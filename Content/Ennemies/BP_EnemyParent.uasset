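; BP_EnemyParent is a base enemy for a tower defense game that walks toward a target and can be killed by damage.
; On BeginPlay it waits briefly, sets its walk speed, then uses AI MoveTo toward the first BP_Target found, destroying itself on arrival.
; AnyDamage subtracts from Life, and at zero the enemy destroys itself and calls AddGold on the BP_TowerController player controller.
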(event EventBeginPlay
  (Utilities|FlowControl|Delay 0.2)
  (Variables|/Script/Engine.CharacterMovementComponent|SetMaxWalkSpeed (Variables|Character|GetCharacterMovement) (Variables|Default|GetspeedMax))
  (bind _outactors (Actor|GetAllActorsOfClass "/Game/LevelElements/SpawnAndTarget/BP_Target.BP_Target_C"))
  (AI|AIMoveTo self "0, 0, 0" (Utilities|Array|Get(acopy) _outactors) 2e+02 false
    (:OnSuccess
      (Actor|DestroyActor))))

(event Game|Damage|EventAnyDamage
  (params (Damage :type Float%20%28single-precision%29) (DamageType :type Damage%20Type%20Object%20Reference) (InstigatedBy :type Controller%20Object%20Reference) (DamageCauser :type Actor%20Object%20Reference))
  (Variables|Default|SetLife (- (Variables|Default|GetLife) Damage))
  (if (<= (Variables|Default|GetLife) 0.0)
    (Actor|DestroyActor)
    (bind _asbp_tower_controller (Utilities|Casting|CastToBP_TowerController (Game|GetPlayerController 0)))
    (Default|AddGold _asbp_tower_controller)))

(fn ConstructionScript)