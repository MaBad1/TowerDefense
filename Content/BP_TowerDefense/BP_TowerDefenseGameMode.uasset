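; Tower defense game mode that runs enemy waves.
; LevelMap reads the current wave's row from DT_VagueDetails into a class-to-count map of DK, Ninja and Boss enemies and totals them.
; A looping timer has a random BP_spawn actor spawn a random type with remaining count, rerolling empty types and decrementing the counts.
; Once none remain to spawn and no BP_EnemyParent actors are alive, it loads the next wave.
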(event Custom|TriggerSpawn
  (bind _spawnlist (Variables|Default|GetSpawnList))
  (if (> (Variables|Default|GetEnemies) 0)
    (bind _enemytospawn (CallFunction|EnemytoSpawn))
    (Default|SpawnEnemy (Utilities|Array|Get(acopy) _spawnlist (Math|Random|RandomIntegerinRange 0 (- (Utilities|Array|Length _spawnlist) 1))) _enemytospawn)
    (else
      ;[1 1 1] Numero de la vague
      (bind _outactors (Actor|GetAllActorsOfClass "/Game/Ennemies/BP_EnemyParent.BP_EnemyParent_C"))
      (if (<= (Utilities|Array|Length _outactors) 0)
        (bind _result (Math|Integer|IncrementInt (Variables|Default|GetWave))
          (:%20%20
            (CallFunction|LevelMap _result)))))))

(event EventBeginPlay
  (bind _outactors (Actor|GetAllActorsOfClass "/Game/LevelElements/SpawnAndTarget/BP_spawn.BP_spawn_C"))
  (Variables|Default|SetSpawnList _outactors)
  (Utilities|Time|SetTimerbyEvent (delegate Custom|TriggerSpawn) 2.0 true)
  (CallFunction|LevelMap (Variables|Default|GetWave)))

(fn ConstructionScript)

(fn LevelMap
  (params (NumeroVague :type Integer))
  (bind _returnvalue (Utilities|GetDataTableRow "/Game/Ennemies/DT_VagueDetails.DT_VagueDetails" (Utilities|String|StringToName (Utilities|String|ToString(Integer) NumeroVague)))
    (:then
      (bind _output_get (Variables|Default|SetEnemyList (Utilities|Map|MakeMap "/Game/Ennemies/BP_EnemyDK.BP_EnemyDK_C" (.dk _returnvalue) "/Game/Ennemies/BP_EnemyNinja.BP_EnemyNinja_C" (.ninja _returnvalue) "/Game/Ennemies/BP_Boss.BP_Boss_C" (.boss _returnvalue))))
      (bind _values (Utilities|Map|Values _output_get))
      (for _array_element _values
        (Variables|Default|SetEnemies (+ _array_element (Variables|Default|GetEnemies)))))))

(fn EnemytoSpawn
  (bind _keys (Utilities|Map|Keys (Variables|Default|GetEnemyList) :!label _label))
  (bind _output_get (Variables|Default|SetSpawningEnemy (Utilities|Array|Get(acopy) _keys (Math|Random|RandomInteger (Utilities|Array|Length _keys)))))
  (Variables|Default|SetEnemyNumber (.Value (Utilities|Map|Find (Variables|Default|GetEnemyList) _output_get)))
  (if (> (.Value (Utilities|Map|Find (Variables|Default|GetEnemyList) _output_get)) 0)
    (Utilities|Map|Add (Variables|Default|GetEnemyList) (Variables|Default|GetSpawningEnemy) (- (Variables|Default|GetEnemyNumber) 1))
    (Variables|Default|SetEnemies (- (Variables|Default|GetEnemies) 1))
    (return (Variables|Default|GetSpawningEnemy))
    (else
      (goto _label))))