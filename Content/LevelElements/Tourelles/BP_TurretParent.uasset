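; Parent turret Blueprint that automatically tracks and fires at enemies entering its overlap volume, with two upgrade steps that change fire rate and mesh.
; Overlap events maintain an in-range list of BP_EnemyParent actors, from which a random target is picked when none is held or the current one leaves.
; A gated, per-frame Delay loop yaws the turret toward the target, while a second Delay paces projectile spawning from the Sphere component.
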(event OnComponentBeginOverlap(OverlapDetect)
  (params (OverlappedComponent :type Primitive%20Component%20Object%20Reference) (OtherActor :type Actor%20Object%20Reference) (OtherComp :type Primitive%20Component%20Object%20Reference) (OtherBodyIndex :type Integer) (bFromSweep :type Boolean) (SweepResult :type Hit%20Result%20Structure%20%28by%20ref%29))
  ;[1 1 1] Detection du début d'overlap et de si l'ennemi est une cible valide
  (bind _asbp_enemy_parent (Utilities|Casting|CastToBP_EnemyParent OtherActor))
  (Utilities|Array|Add (Variables|Default|GetTargetInRange) _asbp_enemy_parent)
  (Utilities|IsValid (Variables|Default|GetTargetDetected)
    (:Is%20Not%20Valid
      (CallFunction|SelectTarget))))

(event OnComponentEndOverlap(OverlapDetect)
  (params (OverlappedComponent :type Primitive%20Component%20Object%20Reference) (OtherActor :type Actor%20Object%20Reference) (OtherComp :type Primitive%20Component%20Object%20Reference) (OtherBodyIndex :type Integer))
  (bind _targetinrange (Variables|Default|GetTargetInRange))
  ;[1 1 1] Detection de la fin d'overlap et changement d'ennemi à cibler + suppression de l'ennemi qui sort du tableau
  (bind _asbp_enemy_parent (Utilities|Casting|CastToBP_EnemyParent OtherActor))
  (if (Utilities|Array|ContainsItem _targetinrange _asbp_enemy_parent)
    (Utilities|Array|RemoveItem _targetinrange _asbp_enemy_parent)
    (if (== (Variables|Default|GetTargetDetected) _asbp_enemy_parent)
      (Variables|Default|SetTargetDetected 0)
      (CallFunction|SelectTarget))))

(event Custom|BeginAim
  ;[1 1 1] Système pour lock un ennemi et tirer en continue tant qu'il est dans l'overlap
  (Utilities|FlowControl|Sequence
    (:then_0
      (goto _label Open))
    (:then_1
      (Utilities|FlowControl|Gate true :!label _label
        (:Exit
          (Utilities|IsValid (Variables|Default|GetTargetDetected)
            (:Is%20Valid
              (Utilities|FlowControl|Sequence
                (:then_0
                  (Utilities|FlowControl|Delay (Variables|Default|GetRateOfFire))
                  (CallFunction|Shoot))
                (:then_1
                  (Variables|Default|SetTargetLocation (Transformation|GetActorLocation (Variables|Default|GetTargetDetected)))
                  (Transformation|SetRelativeRotation (Variables|Default|GetTurret) (Math|Rotator|MakeRotator 0.0 0.0 (.Yaw (Math|Rotator|BreakRotator (Math|Rotator|MakeRotfromX (Math|Transform|InverseTransformDirection (Transformation|GetActorTransform) (- (Variables|Default|GetTargetLocation) (Transformation|GetWorldLocation (Variables|Default|GetTurret)))))))) false false)
                  (Utilities|FlowControl|Delay (Utilities|Time|GetWorldDeltaSeconds))
                  (CallFunction|ContinueAim))))
            (:Is%20Not%20Valid
              (CallFunction|CancelAim))))))))

(event Custom|TurretUpgrade
  ;[1 1 1] Upgrade De Tourelles
  (if (Variables|Default|GetUpgrade1)
    (Variables|Default|SetRateOfFire (Variables|Default|GetRateOfFireV2))
    (Components|StaticMesh|SetStaticMesh (Variables|Default|GetTurret) (Variables|Default|GetTurretV2))
    (Variables|Default|Setupgrade2 true)
    (Variables|Default|SetUpgrade1 false)
    (elif (Variables|Default|Getupgrade2)
      (Variables|Default|SetRateOfFire (Variables|Default|GetRateOfFireV3))
      (Components|StaticMesh|SetStaticMesh (Variables|Default|GetTurret) (Variables|Default|GetTurretV3))
      (Variables|Default|Setupgrade2 false))))

(event Custom|CancelAim
  ;[1 1 1] Système pour lock un ennemi et tirer en continue tant qu'il est dans l'overlap
  (Utilities|FlowControl|Gate true) ; enters at Close
)

(event Custom|SelectTarget
  (bind _targetinrange (Variables|Default|GetTargetInRange))
  ;[1 1 1] Selection de l'ennemi à target
  (if (Utilities|Array|IsValidIndex _targetinrange)
    (Variables|Default|SetTargetDetected (Utilities|Array|Get(acopy) _targetinrange (Math|Random|RandomIntegerinRange 0 (Utilities|Array|LastIndex _targetinrange))))
    (CallFunction|BeginAim)))

(event Custom|ContinueAim
  ;[1 1 1] Système pour lock un ennemi et tirer en continue tant qu'il est dans l'overlap
  (Utilities|IsValid (Variables|Default|GetTargetDetected)
    (:Is%20Valid
      (Utilities|FlowControl|Gate true
        (:Exit
          (Utilities|IsValid (Variables|Default|GetTargetDetected)
            (:Is%20Valid
              (Utilities|FlowControl|Sequence
                (:then_0
                  (Utilities|FlowControl|Delay (Variables|Default|GetRateOfFire))
                  (CallFunction|Shoot))
                (:then_1
                  (Variables|Default|SetTargetLocation (Transformation|GetActorLocation (Variables|Default|GetTargetDetected)))
                  (Transformation|SetRelativeRotation (Variables|Default|GetTurret) (Math|Rotator|MakeRotator 0.0 0.0 (.Yaw (Math|Rotator|BreakRotator (Math|Rotator|MakeRotfromX (Math|Transform|InverseTransformDirection (Transformation|GetActorTransform) (- (Variables|Default|GetTargetLocation) (Transformation|GetWorldLocation (Variables|Default|GetTurret)))))))) false false)
                  (Utilities|FlowControl|Delay (Utilities|Time|GetWorldDeltaSeconds))
                  (CallFunction|ContinueAim))))
            (:Is%20Not%20Valid
              (CallFunction|CancelAim :!label _label))))))
    (:Is%20Not%20Valid
      (goto _label))))

(event EventBeginPlay)

(event Collision|EventActorBeginOverlap
  (params (OtherActor :type Actor%20Object%20Reference)))

(event EventTick
  (params (DeltaSeconds :type Float%20%28single-precision%29)))

(fn ConstructionScript)

(fn Shoot
  (Game|SpawnActorfromClass (Variables|Default|GetAmmoType) (Transformation|GetWorldTransform (Variables|Default|GetSphere)) "Undefined" 0 0)
  (Variables|Default|SetBullet 0))